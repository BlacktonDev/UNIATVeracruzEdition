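; Coconut_BP is a melee enemy character driven by a behavior tree and armed with a sword.
; On begin play it starts the tree, attaches a spawned sword to its socket, hands it to the trace component, caches the player and writes its behaviour enum to the blackboard.
; The Attack event plays a random montage and stores its length.
; Damage reduces health, triggering a hit reaction or a one-time death montage below zero.
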(event `Attack`
  (bind _returnvalue (`self.PlayAnimMontage` (`KismetArrayLibrary.Array_Random` (`self.Attack Animations`))))
  (set `self.Attack Lenght` _returnvalue))

(event `self.ReceiveBeginPlay`
  (`AIController.RunBehaviorTree` (`AIBlueprintHelperLibrary.GetAIController` self) "/Game/_Romo/Enemy/BehaviourTree/CoconutBehaviourTree.CoconutBehaviourTree")
  (bind _returnvalue (`|SpawnActorFromClass` (`self.sword`) (`SceneComponent.GetSocketTransform` (`self.Mesh`) "sword" "RTS_World") "Undefined" "MultiplyWithRoot" null null))
  (bind _asbase_werapon_bp (cast `/Game/_Romo/Enemy/Weapons/BaseWerapon_BP` _returnvalue))
  (bind _output_get (set `self.Weapon Ref` _asbase_werapon_bp))
  (`self.K2_AttachToComponent` _output_get (`self.Mesh`) "sword" "SnapToTarget" "SnapToTarget" "SnapToTarget" true)
  (set `/Game/_Romo/Enemy/Weapons/TraceComponent.Sword  Ref` (`self.Weapon Ref`) (`self.TraceComponent`))
  (bind _asbp_third_person_character (cast `/Game/ThirdPerson/Blueprints/BP_ThirdPersonCharacter` (`GameplayStatics.GetPlayerCharacter` 0)))
  (set `self.Character Reference` _asbp_third_person_character)
  (`BlackboardComponent.SetValueAsEnum` (`AIBlueprintHelperLibrary.GetBlackboard` null) "ebehaviour" (`self.behaviour`)))

(event `self.ReceiveAnyDamage`
  (params (Damage :type "Float (single-precision)") (DamageType :type "DamageType Object Reference") (InstigatedBy :type "Controller Object Reference") (DamageCauser :type "Actor Object Reference"))
  (bind _output_get (set `self.Health` (- (`self.Health`) Damage)))
  (`KismetSystemLibrary.PrintString` (`KismetStringLibrary.Conv_DoubleToString` _output_get))
  (if (< _output_get 0.0)
    (`/Engine/EditorBlueprintResources/StandardMacros.DoOnce` false
      (:`Completed`
        ;[0.9473 0 1 0.3765] Animaciones
        (`self.PlayAnimMontage` "/Game/_Romo/Enemy/Animations/SkeleDeath_Montage.SkeleDeath_Montage") ; Animación de muerte
      ))
    (else
      (`self.PlayAnimMontage` "/Game/_Romo/Enemy/Animations/Skele_Hit_Montage.Skele_Hit_Montage") ; Animación de recibir daño
    )))

(fn `UserConstructionScript`)