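; MegaCoconut boss enemy with sword melee and projectile attacks, driven by a behavior tree.
; On begin play it attaches a spawned sword, wires it to the trace component and targets the player with a rotating component.
; First sighting of the player shows a health bar and switches the blackboard behaviour.
; Two damage events reduce health; death stops AI logic, plays a montage, disables capsule collision and removes the bar.
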(event `Attack`
  ;[1 1 1] Ataque
  (bind _returnvalue (`self.PlayAnimMontage` (`KismetArrayLibrary.Array_Random` (`self.Attack Animations`))))
  (set `self.Attack Lenght` _returnvalue))

(event `self.ReceiveBeginPlay`
  ;[1 1 1] Inicio
  (set `self.MaxHealth` (`self.Health`))
  (`AIController.RunBehaviorTree` (`AIBlueprintHelperLibrary.GetAIController` self) "/Game/_Romo/Enemy/Boss/Behaviour_Tree/MegaCoconut_BT.MegaCoconut_BT")
  (bind _returnvalue (`|SpawnActorFromClass` (`self.sword`) (`SceneComponent.GetSocketTransform` (`self.Mesh`) "sword" "RTS_World") "Undefined" "MultiplyWithRoot" null null))
  (bind _output_get (set `self.Weapon Ref` _returnvalue))
  (`self.K2_AttachToComponent` _output_get (`self.Mesh`) "sword" "SnapToTarget" "SnapToTarget" "SnapToTarget" true)
  (set `/Game/_Romo/Enemy/Weapons/TraceComponent.Sword  Ref` (`self.Weapon Ref`) (`self.TraceComponent`))
  (bind _asbp_third_person_character (cast `/Game/ThirdPerson/Blueprints/BP_ThirdPersonCharacter` (`GameplayStatics.GetPlayerCharacter` 0)))
  (set `self.Character Reference` _asbp_third_person_character)
  (`BlackboardComponent.SetValueAsEnum` (`AIBlueprintHelperLibrary.GetBlackboard` null) "ebehaviour" (`self.behaviour`))
  (set `/Game/_Romo/Enemy/Weapons/RotatingComponent.Target` (`GameplayStatics.GetPlayerCharacter` 0) (`self.RotatingComponent`))
  (bind _outactors (`GameplayStatics.GetAllActorsWithTag` "enemy"))
  (set `/Game/_Romo/Enemy/Weapons/TraceComponent.Enemy` _outactors (`self.TraceComponent`)))

(event `self.ReceiveAnyDamage`
  (params (Damage :type "Float (single-precision)") (DamageType :type "DamageType Object Reference") (InstigatedBy :type "Controller Object Reference") (DamageCauser :type "Actor Object Reference"))
  (bind _megacocohealthbar (`self.MegaCocoHealthBar`))
  ;[0.9473 0 1 0.3765] Damage
  (bind _output_get (set `self.Health` (- (`self.Health`) Damage)))
  (`/Engine/EditorBlueprintResources/StandardMacros.IsValid` _megacocohealthbar
    (:`Is Valid`
      (`/Game/_Romo/Enemy/Boss/MegaCocoHealthBar_WB.Update Health Bar` _megacocohealthbar)
      (if (<= _output_get 0.0)
        (`/Engine/EditorBlueprintResources/StandardMacros.DoOnce` false
          (:`Completed`
            (`BrainComponent.StopLogic` (`AIController.BrainComponent` (`AIBlueprintHelperLibrary.GetAIController` self)) "die")
            (`self.PlayAnimMontage` "/Game/_Romo/Enemy/Boss/Animations/MegaCocoDeathDeath_Montage.MegaCocoDeathDeath_Montage")
            (`PrimitiveComponent.SetCollisionEnabled` (`self.CapsuleComponent`) "NoCollision")
            (`ActorComponent.K2_DestroyComponent` (`self.CharacterMovement`))
            (`Widget.RemoveFromParent` (`self.MegaCocoHealthBar`))))))))

(event `self.PawnSensing.OnSeePawn`
  (params (Pawn :type "Pawn Object Reference"))
  ;[1 1 1] Enemy vision
  (if (== Pawn (`GameplayStatics.GetPlayerCharacter` 0))
    (`/Engine/EditorBlueprintResources/StandardMacros.DoOnce` false
      (:`Completed`
        (bind _returnvalue (`|CreateWidget` "/Game/_Romo/Enemy/Boss/MegaCocoHealthBar_WB.MegaCocoHealthBar_WB_C" null self))
        (bind _output_get (set `self.MegaCocoHealthBar` _returnvalue))
        (`UserWidget.AddToViewport` _output_get 0)
        (set `self.behaviour` "NewEnumerator3")
        (`BlackboardComponent.SetValueAsEnum` (`AIBlueprintHelperLibrary.GetBlackboard` null) "ebehaviour" (`self.behaviour`))))))

(event `Projectile Attack`
  ;[1 1 1] Projectile Attack
  (bind _returnvalue (`self.PlayAnimMontage` "/Game/_Romo/Enemy/Boss/Animations/BossRangedAttack.BossRangedAttack"))
  (set `self.Ranged Attack Lenght` _returnvalue))

(event `Clear Hit Actors`
  ;[1 1 1] Clear hit actors, para que le vuelva a pegar
  (`KismetArrayLibrary.Array_Clear` (`/Game/_Romo/Enemy/Weapons/TraceComponent.actorstoignore` (`self.TraceComponent`))))

(event `Fire Projectile`
  (bind _returnvalue (`SceneComponent.K2_GetComponentLocation` (`self.ProjectileSpawnPoint`)))
  ;[1 1 1] Shoot
  (`|SpawnActorFromClass` "/Game/_Romo/Enemy/Boss/MegaCocoProjectile_BP.MegaCocoProjectile_BP_C" (`KismetMathLibrary.MakeTransform` _returnvalue (`KismetMathLibrary.FindLookAtRotation` _returnvalue (`self.K2_GetActorLocation` (`GameplayStatics.GetPlayerCharacter` 0)))) "Undefined" "MultiplyWithRoot" null null))

(event `/Game/Progra/Player/BPI_Damageable.I_TakeDamage`
  (params (Damage :type "Float (double-precision)"))
  (bind _megacocohealthbar (`self.MegaCocoHealthBar`))
  ;[0.9473 0 1 0.3765] Damage
  (bind _output_get (set `self.Health` (- (`self.Health`) Damage)))
  (`/Engine/EditorBlueprintResources/StandardMacros.IsValid` _megacocohealthbar
    (:`Is Valid`
      (`/Game/_Romo/Enemy/Boss/MegaCocoHealthBar_WB.Update Health Bar` _megacocohealthbar)
      (if (<= _output_get 0.0)
        (`/Engine/EditorBlueprintResources/StandardMacros.DoOnce` false
          (:`Completed`
            (`BrainComponent.StopLogic` (`AIController.BrainComponent` (`AIBlueprintHelperLibrary.GetAIController` self)) "die")
            (`self.PlayAnimMontage` "/Game/_Romo/Enemy/Boss/Animations/MegaCocoDeathDeath_Montage.MegaCocoDeathDeath_Montage")
            (`PrimitiveComponent.SetCollisionEnabled` (`self.CapsuleComponent`) "NoCollision")
            (`ActorComponent.K2_DestroyComponent` (`self.CharacterMovement`))
            (`Widget.RemoveFromParent` (`self.MegaCocoHealthBar`))))))))

(fn `UserConstructionScript`)