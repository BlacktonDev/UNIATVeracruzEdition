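; BP_Smg is the player's SMG, a child gun Blueprint that snaps to the GripPoint socket on the player mesh at BeginPlay.
; IShoot activates the GunSpray particle emitter and starts a looping timer that removes one bullet every FiringDelay.
; IStopShooting deactivates the spray and clears the timer; an empty magazine triggers it automatically, followed by IShotAttempt.
; The Tick subtraction is zero, so only the timer drains ammo.
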(event `self.ReceiveBeginPlay`
  (`parent.ReceiveBeginPlay`)
  (`self.K2_AttachToComponent` (`Character.Mesh` (`self.Player`)) "GripPoint" "SnapToTarget" "SnapToTarget" "KeepRelative"))

(event `self.ReceiveTick`
  (params (DeltaSeconds :type "Float (single-precision)"))
  (`parent.ReceiveTick` DeltaSeconds)
  (if (`self.isShooting`)
    (set `self.BulletCount` (- (`self.BulletCount`) 0.0))))

(event `self.I_Shoot`
  ;[1 1 1] Receive input from player
  ;[0 1 0] We are now shooting
  (set `self.isShooting` true)
  ;[0 1 0] Start the particle emitter
  (`ActorComponent.Activate` (`self.GunSpray`) false)
  (bind _returnvalue (`KismetSystemLibrary.K2_SetTimerDelegate` (delegate `ReduceAmmo`) (`self.FiringDelay`) true)))

(event `ReduceAmmo`
  (if (> (`self.BulletCount`) 0.0)
    (set `self.BulletCount` (- (`self.BulletCount`) 1.0))
    (else
      (`self.I_StopShooting`)
      (`self.I_ShotAttempt`))))

(event `self.I_StopShooting`
  ;[1 0 0] We are no longer shooting
  (set `self.isShooting` false)
  ;[1 0 0] Stop the particle emitter
  (`ActorComponent.Deactivate` (`self.GunSpray`))
  (`KismetSystemLibrary.K2_ClearAndInvalidateTimerHandle` (stale `self.I_Shoot` _returnvalue)))

(fn `UserConstructionScript`
  (`parent.UserConstructionScript`))