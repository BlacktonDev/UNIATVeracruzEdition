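; BP_AmbientSound is a placeable ambient sound emitter that starts playing when the third-person character enters its trigger sphere.
; The construction script applies the sound cue, attenuation settings and sphere radius variables to the audio and collision components.
; On overlap, playback starts at a random offset within the cue's duration, while other actors only trigger a debug message.
; The graph has no end-overlap handling to stop the sound.
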(event `self.SphereCol.OnComponentBeginOverlap`
  (params (OverlappedComponent :type "PrimitiveComponent Object Reference") (OtherActor :type "Actor Object Reference") (OtherComp :type "PrimitiveComponent Object Reference") (OtherBodyIndex :type Integer) (bFromSweep :type Boolean) (SweepResult :type "HitResult Structure (by ref)"))
  (cast `/Game/ThirdPerson/Blueprints/BP_ThirdPersonCharacter` OtherActor
    (:`then`
      (`AudioComponent.Play` (`self.AmbientSoundAudio`) (`KismetMathLibrary.RandomFloatInRange` 0.0 (`SoundBase.Duration` (`self.SounCue`)))))
    (:`CastFailed`
      (`KismetSystemLibrary.PrintString` "Cast of ambient sound failed" true true (struct :`R` 1.0 :`B` 0.094506 :`A` 1.0) 10.0))))

(fn `UserConstructionScript`
  (bind _ambientsoundaudio (`self.AmbientSoundAudio`))
  (`AudioComponent.SetSound` _ambientsoundaudio (`self.SounCue`))
  (set `AudioComponent.AttenuationSettings` (`self.AmbientSounAttenuation`) _ambientsoundaudio)
  (`SphereComponent.SetSphereRadius` (`self.SphereCol`) (`self.SphereRadius`) true))